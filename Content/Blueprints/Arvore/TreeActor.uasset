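; Choppable tree actor that counts hits through a rising Hardness value, then slices itself and falls under physics.
; The construction script copies the static TreeMesh into the procedural CutTree mesh.
; Each valid InteractTree raises Hardness on a dynamic trunk material; the first also spawns a BpCutTree above the actor.
; At the threshold, it resets Hardness, swaps to CutTree, slices it along a tilted plane and enables physics.
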(event EventBeginPlay
  (bind _returnvalue (Rendering|Material|CreateDynamicMaterialInstance "/Game/Blueprints/Arvore/Material/M_TreeTrunk_Inst.M_TreeTrunk_Inst" "None" "None" :!class /Script/Engine.KismetMaterialLibrary))
  (bind _output_get (Variables|Default|SetTreeMaterial _returnvalue))
  (Rendering|Material|SetMaterial (Variables|Default|GetTreeMesh) 0 _output_get)
  (Collision|SetCollisionEnabled (Variables|Default|GetCutTree) "QueryAndPhysics"))

(event EventInteractTree
  (params (Player :type Actor%20Object%20Reference) (IsValid :type Boolean))
  (bind _returnvalue (Transformation|GetActorLocation))
  (bind _treemesh (Variables|Default|GetTreeMesh))
  (bind _cuttree (Variables|Default|GetCutTree))
  (bind _returnvalue_2 (Transformation|GetWorldLocation _treemesh))
  (if IsValid
    (Utilities|FlowControl|Sequence
      (:then_0
        (Utilities|FlowControl|DoOnce false
          (:Completed
            (Game|SpawnActorfromClass "/Game/Blueprints/Arvore/BpCutTree.BpCutTree_C" (Math|Transform|MakeTransform (Math|Vector|MakeVector (.x _returnvalue) (.y _returnvalue) (+ (.z _returnvalue) 115.0)) "0, 0, 0" "1.000000,1.000000,1.000000") "Undefined" "MultiplyWithRoot" 0 0))))
      (:then_1
        (if (>= (Variables|Default|GetHardness) 0.4)
          (Variables|Default|SetHardness -1.0)
          (Development|PrintString "Cortar")
          (Rendering|SetVisibility (Variables|Default|GetTreeMesh) false false)
          (Rendering|SetVisibility (Variables|Default|GetCutTree) true false)
          (Class|KismetProceduralMeshLibrary|SliceProceduralMesh (Variables|Default|GetCutTree) (Math|Vector|MakeVector (.x _returnvalue_2) (.y _returnvalue_2) (+ (.z _returnvalue_2) 1.1e+02)) (Math|Vector|MakeVector 0.2 0.2 0.9) true "UseLastSectionForCap")
          (Physics|SetSimulatePhysics _cuttree true)
          (Physics|SetEnableGravity _cuttree true)
          (Rendering|Material|SetMaterial _cuttree 0 "/Game/Blueprints/Arvore/Material/M_TreeTrunk_Inst.M_TreeTrunk_Inst")
          (else
            (Development|PrintString "Bateu")
            (bind _output_get (Variables|Default|SetHardness (+ (Variables|Default|GetHardness) 0.1)))
            (Rendering|Material|SetScalarParameterValue (Variables|Default|GetTreeMaterial) "Hardness" _output_get :!class /Script/Engine.MaterialInstanceDynamic)))))))

(fn ConstructionScript
  (Class|KismetProceduralMeshLibrary|CopyProceduralMeshfromStaticMeshComponent (Variables|Default|GetTreeMesh) 0 (Variables|Default|GetCutTree) false))